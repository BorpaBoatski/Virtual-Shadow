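; BP_PropsSpawner streams random rock and tree props around the Bus as it travels along Y in the road scene.
; A virtual Y cursor advances tile by tile, staying a set range ahead of the Bus.
; Each row places props at random tile offsets across two X ranges, adding instances to one of four instanced mesh components.
; Tick removes the oldest instance once far behind, but only for Rock1.
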(event EventBeginPlay
  ;[1 1 1] Set the origin of spawner to Bus position
  (Transformation|SetActorLocation (Transformation|GetActorLocation (Variables|Default|GetBus)) false false)
  (Variables|Default|SetVirtualPosY (- (.Y (Math|Vector|BreakVector (Transformation|GetActorLocation))) (Variables|Default|GetHorizontalRange)))
  (while (<= (- (Variables|Default|GetVirtualPosY) (.Y (Math|Vector|BreakVector (Transformation|GetActorLocation (Variables|Default|GetBus))))) (Variables|Default|GetHorizontalRange))
    (CallFunction|PopulatePropsAlongX)
    (CallFunction|GotoNextPosY)))

(event EventTick
  (params (DeltaSeconds :type Float%20%28single-precision%29))
  (bind _rock1 (Variables|Default|GetRock1))
  (bind (_outinstancetransform _returnvalue) (Components|InstancedStaticMesh|GetInstanceTransform _rock1 0 true))
  (while (<= (- (Variables|Default|GetVirtualPosY) (.Y (Math|Vector|BreakVector (Transformation|GetActorLocation (Variables|Default|GetBus))))) (Variables|Default|GetHorizontalRange))
    (CallFunction|PopulatePropsAlongX)
    (CallFunction|GotoNextPosY))
  ;[1 1 1] Remove the eldest prop if condition is fulfilled
  (if _returnvalue
    (if (>= (- (.Y (Math|Vector|BreakVector (Transformation|GetActorLocation (Variables|Default|GetBus)))) (.Y (Math|Vector|BreakVector (.Location (Math|Transform|BreakTransform _outinstancetransform))))) (Variables|Default|GetHorizontalRange))
      (Class|InstancedStaticMeshComponent|RemoveInstance (Variables|Default|GetRock1)))))

(fn ConstructionScript)

(fn PopulatePropsAlongX
  (bind _output_get (LocalVariables|Set_NumOfProp (Math|Random|RandomIntegerinRange 0 4)))
  (LocalVariables|Set_CachedIndex 0)
  (for _index (range 0 _output_get)
    (bind _output_get_2 (LocalVariables|Set_CachedIndex (+ (LocalVariables|Get_CachedIndex) (Math|Random|RandomIntegerinRange 0 4))))
    (bind _output_get_3 (LocalVariables|Set_SpawnPosX (+ (Variables|Default|GetMinRangeX1) (* _output_get_2 (Variables|Default|GetTileSize)))))
    (if (>= _output_get_3 (Variables|Default|GetMaxRangeX1))
      (bind _output_get_4 (LocalVariables|Set_SpawnPosX (+ (- (Variables|Default|GetMaxRangeX1) (LocalVariables|Get_SpawnPosX)) (Variables|Default|GetMinRangeX2))))
      (CallFunction|AddPropsInst (Math|Transform|MakeTransform (Math|Vector|MakeVector _output_get_4 (Variables|Default|GetVirtualPosY) (.Z (Math|Vector|BreakVector (Transformation|GetActorLocation))))))
      (else
        (CallFunction|AddPropsInst (Math|Transform|MakeTransform (Math|Vector|MakeVector _output_get_3 (Variables|Default|GetVirtualPosY) (.Z (Math|Vector|BreakVector (Transformation|GetActorLocation))))))))))

(fn GotoNextPosY
  (Variables|Default|SetVirtualPosY (+ (Variables|Default|GetVirtualPosY) (Variables|Default|GetTileSize))))

(fn AddPropsInst
  (params (SpawnXForm :type Transform))
  (switch int (Math|Random|RandomIntegerinRange 0 3)
    (:0
      (Components|InstancedStaticMesh|AddInstance (Variables|Default|GetRock1) SpawnXForm))
    (:1
      (Components|InstancedStaticMesh|AddInstance (Variables|Default|GetTree1) SpawnXForm))
    (:2
      (Components|InstancedStaticMesh|AddInstance (Variables|Default|GetTree2) SpawnXForm))
    (:3
      (Components|InstancedStaticMesh|AddInstance (Variables|Default|GetTree3) SpawnXForm))))