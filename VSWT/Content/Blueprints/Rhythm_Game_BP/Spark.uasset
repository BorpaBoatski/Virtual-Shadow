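; Spark is a short-lived particle effect actor in the rhythm game that shows a colored spark and destroys itself after a brief delay.
; On BeginPlay it passes its ColorFloat value to DetermineColor, which maps three value bands to green, blue or red.
; The chosen color is written to the particle system's InitialColor and SparkColor parameters.
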(event EventBeginPlay
  (CallFunction|DetermineColor (Variables|Default|GetColorFloat))
  (Utilities|FlowControl|Delay 0.3)
  (Actor|DestroyActor))

(fn ConstructionScript)

(fn DetermineColor
  (params (ColorInt :type Float%20%28single-precision%29))
  (bind _particlesystem (Variables|Default|GetParticleSystem))
  (if (< ColorInt 1e+01)
    (Variables|Default|SetColor (Math|Conversions|ToColor(LinearColor) (Math|Color|MakeColor 0.0 1.0 0.0)))
    (Effects|Components|ParticleSystem|SetColorParameter _particlesystem "InitialColor" (Math|Conversions|ToLinearColor(Color) (Variables|Default|GetColor)) :!label _label)
    (Effects|Components|ParticleSystem|SetColorParameter _particlesystem "SparkColor" (Math|Conversions|ToLinearColor(Color) (Variables|Default|GetColor)))
    (elif (>= ColorInt 15.0)
      (Variables|Default|SetColor (Math|Conversions|ToColor(LinearColor) (Math|Color|MakeColor 1.0 0.0 0.0)))
      (goto _label)
      (elif (>= ColorInt 1e+01)
        (Variables|Default|SetColor (Math|Conversions|ToColor(LinearColor) (Math|Color|MakeColor 0.0 0.0 1.0)))
        (goto _label)))))