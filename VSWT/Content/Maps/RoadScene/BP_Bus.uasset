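; BP_Bus is the bus in the road scene, driving forward while an isometric camera tracks it.
; On BeginPlay it makes IsometricCamera the view target, places CameraBase on the bus and starts departing.
; Tick ramps speed up to MaxSpeed or down to zero, driven by StartBus and StopBus flags.
; CameraBase waits until the bus moves far enough along Y, then eases toward an offset position using VInterpTo.
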(event EventBeginPlay
  ;[1 1 1] Set the assigned IsoCamera as the main camera
  (Game|Player|SetViewTargetwithBlend (Game|GetPlayerController 0) (Variables|Default|GetIsometricCamera) 0.0 "VTBlend_Linear" 0.0 false)
  ;[1 1 1] The camera starts at the same position of the Bus, then moves to the front of bus during frame updates
  (Transformation|SetActorLocation (Variables|Default|GetCameraBase) (Transformation|GetActorLocation) false false)
  (CallFunction|StartBus))

(event EventTick
  (params (DeltaSeconds :type Float%20%28single-precision%29))
  (bind _returnvalue (Transformation|GetActorLocation))
  (bind _camerabase (Variables|Default|GetCameraBase))
  (bind _returnvalue_2 (Transformation|GetActorLocation _camerabase))
  ;[1 1 1] Accelerates
  (if (Variables|Default|GetbDeparting)
    (bind _output_get (Variables|Default|SetTravelSpeed (+ (Variables|Default|GetTravelSpeed) (* (Variables|Default|GetAccel) DeltaSeconds))))
    (if (> _output_get (Variables|Default|GetMaxSpeed))
      (Variables|Default|SetbDeparting false)
      (Variables|Default|SetTravelSpeed (Variables|Default|GetMaxSpeed)))
    (else
      ;[1 1 1] Decelerates
      (if (Variables|Default|GetbStopping)
        (bind _output_get_2 (Variables|Default|SetTravelSpeed (- (Variables|Default|GetTravelSpeed) (* (Variables|Default|GetAccel) DeltaSeconds))))
        (if (< _output_get_2 0.0)
          (Variables|Default|SetbStopping false)
          (Variables|Default|SetTravelSpeed 0.0)))))
  ;[1 1 1] Moves Bus Forward
  (Transformation|SetActorLocation (+ (Transformation|GetActorLocation) (* (Transformation|GetActorForwardVector) (* DeltaSeconds (Variables|Default|GetTravelSpeed)))) false false)
  ;[1 1 1] Implements Camera Follow Bus
  (if (Variables|Default|GetbCameraFollow)
    (Transformation|SetActorLocation _camerabase (Math|Interpolation|VInterpTo _returnvalue_2 (+ _returnvalue (Variables|Default|GetCameraBaseOffset)) DeltaSeconds 0.75) false false)
    (else
      (Variables|Default|SetbCameraFollow (>= (.Y (Math|Vector|BreakVector (- _returnvalue _returnvalue_2))) (stale _result))))))

(fn ConstructionScript)

(fn StopBus
  (Variables|Default|SetbStopping true))

(fn StartBus
  (Variables|Default|SetbDeparting true))