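; Four-lane rhythm minigame board that spawns colored notes to music and pays points out as GameInstance money before loading the shop level.
; Tick compares world time against MusicScore keys, spawning notes ahead of their timestamps and consuming each entry.
; D/F/J/K raise plucks with brief overlap windows, scoring hits by proximity plus combo.
; Notes reaching DeadEnd drain health, pausing into game over at zero.
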(event OnComponentBeginOverlap(DeadEnd)
  (params (OverlappedComponent :type Primitive%20Component%20Object%20Reference) (OtherActor :type Actor%20Object%20Reference) (OtherComp :type Primitive%20Component%20Object%20Reference) (OtherBodyIndex :type Integer) (bFromSweep :type Boolean) (SweepResult :type Hit%20Result%20Structure%20%28by%20ref%29))
  ;[1 1 1] Health System
  (if (== (Utilities|GetClass OtherActor) "/Game/Blueprints/Rhythm_Game_BP/Note_BP.Note_BP_C")
    (Variables|Default|SetHealth (- (Variables|Default|GetHealth) 1.0))
    (Variables|Default|SetCombo 0)
    (Actor|DestroyActor OtherActor)
    (if (== (Variables|Default|GetHealth) 0.0)
      (Game|SetGamePaused true)
      (bind _returnvalue (UserInterface|CreateWidget "/Game/Blueprints/Rhythm_Game_BP/Rhythm_GameOver.Rhythm_GameOver_C" (Game|GetPlayerController 0)))
      (UserInterface|Viewport|AddtoViewport _returnvalue 0))))

(event OnComponentBeginOverlap(Pluck1)
  (params (OverlappedComponent :type Primitive%20Component%20Object%20Reference) (OtherActor :type Actor%20Object%20Reference) (OtherComp :type Primitive%20Component%20Object%20Reference) (OtherBodyIndex :type Integer) (bFromSweep :type Boolean) (SweepResult :type Hit%20Result%20Structure%20%28by%20ref%29))
  ;[1 1 1] Pluck 1 Detection
  (CallFunction|CheckHit OtherActor (Variables|Default|GetPluck1)))

(event OnComponentBeginOverlap(Pluck2)
  (params (OverlappedComponent :type Primitive%20Component%20Object%20Reference) (OtherActor :type Actor%20Object%20Reference) (OtherComp :type Primitive%20Component%20Object%20Reference) (OtherBodyIndex :type Integer) (bFromSweep :type Boolean) (SweepResult :type Hit%20Result%20Structure%20%28by%20ref%29))
  ;[1 1 1] Pluck 2 Detection
  (CallFunction|CheckHit OtherActor (Variables|Default|GetPluck2)))

(event OnComponentBeginOverlap(Pluck3)
  (params (OverlappedComponent :type Primitive%20Component%20Object%20Reference) (OtherActor :type Actor%20Object%20Reference) (OtherComp :type Primitive%20Component%20Object%20Reference) (OtherBodyIndex :type Integer) (bFromSweep :type Boolean) (SweepResult :type Hit%20Result%20Structure%20%28by%20ref%29))
  ;[1 1 1] Pluck 3 Detection
  (CallFunction|CheckHit OtherActor (Variables|Default|GetPluck3)))

(event OnComponentBeginOverlap(Pluck4)
  (params (OverlappedComponent :type Primitive%20Component%20Object%20Reference) (OtherActor :type Actor%20Object%20Reference) (OtherComp :type Primitive%20Component%20Object%20Reference) (OtherBodyIndex :type Integer) (bFromSweep :type Boolean) (SweepResult :type Hit%20Result%20Structure%20%28by%20ref%29))
  ;[1 1 1] Pluck 4 Detection
  (CallFunction|CheckHit OtherActor (Variables|Default|GetPluck4)))

(event EventBeginPlay
  ;[1 1 1] Init
  (CallFunction|GetSpawnPoints)
  (bind _returnvalue (UserInterface|CreateWidget "/Game/Blueprints/Rhythm_Game_BP/Rhythm_HUD.Rhythm_HUD_C" (Game|GetPlayerController 0)))
  (UserInterface|Viewport|AddtoViewport _returnvalue 0))

(event EventTick
  (params (DeltaSeconds :type Float%20%28single-precision%29))
  (bind _musicscore (Variables|Default|GetMusicScore))
  ;[1 1 1] Spawn when timing is reached
  (if (Audio|Components|Audio|IsPlaying (Variables|Default|GetAudio))
    (bind _output_get (Variables|Default|SetSongPosition (Utilities|Time|GetTimeSeconds)))
    (if (> (Utilities|Map|Length (Variables|Default|GetMusicScore)) 0)
      (bind _keys (Utilities|Map|Keys _musicscore))
      (if (>= _output_get (- (Utilities|Array|Get(acopy) _keys) 2.8))
        (CallFunction|SpawnNote (.Value (Utilities|Map|Find _musicscore (Utilities|Array|Get(acopy) _keys))))))
    (elif (not (Variables|Default|GetIsEnd))
      (Variables|Default|SetIsEnd true)
      (CameraFades|StartCameraFade :self (Game|GetPlayerCameraManager 0) :FromAlpha 0.0 :ToAlpha 1.0 :Duration 2.0 :bShouldFadeAudio true :bHoldWhenFinished true)
      (Widget|SetVisibility (stale EventBeginPlay _returnvalue) "Hidden")
      (Utilities|FlowControl|Delay 3.0)
      (bind _asmy_game_instance (Utilities|Casting|CastToMyGameInstance (Game|GetGameInstance)))
      (Variables|/Game/MyGameInstance.MyGameInstance_C|SetMoney _asmy_game_instance (+ (Variables|/Game/MyGameInstance.MyGameInstance_C|GetMoney _asmy_game_instance) (Variables|Default|GetPoints)))
      (Game|OpenLevel(byName) "LevelShopBP"))))

(event Input|KeyboardEvents|K
  (params (Key :type Key%20Structure))
  (bind _pluck4 (Variables|Default|GetPluck4))
  ;[1 1 1] Lift/Drop Pluck4
  (:Pressed
    (CallFunction|Pluck _pluck4 true)
    (Audio|Components|Audio|Play (Variables|Default|GetSFX4) 0.0)
    (Utilities|FlowControl|Delay 0.2)
    (Variables|/Script/Engine.PrimitiveComponent|SetbGenerateOverlapEvents _pluck4 false))
  (:Released
    (CallFunction|Pluck _pluck4 false)))

(event Input|KeyboardEvents|D
  (params (Key :type Key%20Structure))
  (bind _pluck1 (Variables|Default|GetPluck1))
  ;[1 1 1] Lift/Drop Pluck1
  (:Pressed
    (CallFunction|Pluck _pluck1 true)
    (Audio|Components|Audio|Play (Variables|Default|GetSFX1) 0.0)
    (Utilities|FlowControl|Delay 0.2)
    (Variables|/Script/Engine.PrimitiveComponent|SetbGenerateOverlapEvents _pluck1 false))
  (:Released
    (CallFunction|Pluck _pluck1 false)))

(event Input|KeyboardEvents|J
  (params (Key :type Key%20Structure))
  (bind _pluck3 (Variables|Default|GetPluck3))
  ;[1 1 1] Lift/Drop Pluck3
  (:Pressed
    (CallFunction|Pluck _pluck3 true)
    (Audio|Components|Audio|Play (Variables|Default|GetSFX3) 0.0)
    (Utilities|FlowControl|Delay 0.2)
    (Variables|/Script/Engine.PrimitiveComponent|SetbGenerateOverlapEvents _pluck3 false))
  (:Released
    (CallFunction|Pluck _pluck3 false)))

(event Input|KeyboardEvents|F
  (params (Key :type Key%20Structure))
  (bind _pluck2 (Variables|Default|GetPluck2))
  ;[1 1 1] Lift/Drop Pluck2
  (:Pressed
    (CallFunction|Pluck _pluck2 true)
    (Audio|Components|Audio|Play (Variables|Default|GetSFX2) 0.0)
    (Utilities|FlowControl|Delay 0.2)
    (Variables|/Script/Engine.PrimitiveComponent|SetbGenerateOverlapEvents _pluck2 false))
  (:Released
    (CallFunction|Pluck _pluck2 false)))

(fn ConstructionScript)

(fn GetSpawnPoints
  (Variables|Default|SetSpawnPoints (Utilities|Array|MakeArray (Transformation|GetWorldTransform (Variables|Default|GetArrow1)) (Transformation|GetWorldTransform (Variables|Default|GetArrow2)) (Transformation|GetWorldTransform (Variables|Default|GetArrow3)) (Transformation|GetWorldTransform (Variables|Default|GetArrow4)))))

(fn SpawnNote
  (params (SpawnPoint :type Integer))
  (bind _musicscore (Variables|Default|GetMusicScore))
  (bind _returnvalue (Game|SpawnActorfromClass "/Game/Blueprints/Rhythm_Game_BP/Note_BP.Note_BP_C" (Utilities|Array|Get(acopy) (Variables|Default|GetSpawnPoints) SpawnPoint) "Undefined" 0 0))
  (if (== SpawnPoint 0)
    (Rendering|Material|SetMaterial (Variables|/Script/Engine.StaticMeshActor|GetStaticMeshComponent _returnvalue) 0 "/Game/Material/BlueTile_Mat.BlueTile_Mat")
    (if (> (Utilities|Map|Length (Variables|Default|GetMusicScore)) 0) :!label _label
      (bind _keys (Utilities|Map|Keys _musicscore))
      (Utilities|Map|Remove _musicscore (Utilities|Array|Get(acopy) _keys)))
    (elif (== SpawnPoint 1)
      (Rendering|Material|SetMaterial (Variables|/Script/Engine.StaticMeshActor|GetStaticMeshComponent _returnvalue) 0 "/Game/Material/GreenTile_Mat.GreenTile_Mat")
      (goto _label)
      (elif (== SpawnPoint 2)
        (Rendering|Material|SetMaterial (Variables|/Script/Engine.StaticMeshActor|GetStaticMeshComponent _returnvalue) 0 "/Game/Material/PinkTile_Mat.PinkTile_Mat")
        (goto _label)
        (elif (== SpawnPoint 3)
          (Rendering|Material|SetMaterial (Variables|/Script/Engine.StaticMeshActor|GetStaticMeshComponent _returnvalue) 0 "/Game/Material/YellowTile_Mat.YellowTile_Mat")
          (goto _label))))))

(fn Pluck
  (params (Pluck :type Static%20Mesh%20Component%20Object%20Reference) (isOn :type Boolean))
  (if isOn
    (Variables|Default|SetFingers (+ (Variables|Default|GetFingers) 1))
    (Variables|/Script/Engine.PrimitiveComponent|SetbGenerateOverlapEvents Pluck true)
    (Transformation|SetWorldLocation Pluck (+ (Transformation|GetWorldLocation Pluck) "0,0.000000,30.000000") false false)
    (else
      (Variables|Default|SetFingers (- (Variables|Default|GetFingers) 1))
      (Variables|/Script/Engine.PrimitiveComponent|SetbGenerateOverlapEvents Pluck false)
      (Transformation|SetWorldLocation Pluck (+ (Transformation|GetWorldLocation Pluck) "0,0.000000,-30.000000") false false)
      (if (== (Variables|Default|GetFingers) 0)
        (if (Variables|Default|GetIsOverlap)
          (Variables|Default|SetIsOverlap false)
          (else
            (Variables|Default|SetCombo 0)))
        (elif (not (Variables|Default|GetIsOverlap))
          (Variables|Default|SetCombo 0))))))

(fn CheckHit
  (params (OtherActor :type Actor%20Object%20Reference) (Pluck :type Static%20Mesh%20Component%20Object%20Reference))
  (bind _returnvalue (Transformation|GetActorLocation OtherActor))
  (bind _returnvalue_2 (Transformation|GetWorldLocation Pluck))
  (bind _returnvalue_3 (- _returnvalue _returnvalue_2))
  (bind _returnvalue_4 (Math|Vector|VectorLength _returnvalue_3))
  (if (== (Utilities|GetClass OtherActor) "/Game/Blueprints/Rhythm_Game_BP/Note_BP.Note_BP_C")
    (Variables|Default|SetIsOverlap true)
    (Variables|/Script/Engine.PrimitiveComponent|SetbGenerateOverlapEvents Pluck false)
    (bind _output_get (Variables|Default|SetCombo (+ (Variables|Default|GetCombo) 1)))
    (Variables|Default|SetPoints (+ (+ (Variables|Default|GetPoints) (Math|Float|Truncate (/ (Variables|Default|GetMaxPoint) _returnvalue_4))) _output_get))
    (Game|SpawnActorfromClass "/Game/Blueprints/Rhythm_Game_BP/Spark.Spark_C" (Math|Conversions|ToTransform(Vector) _returnvalue) "Undefined" 0 _returnvalue_4 0)
    (Actor|DestroyActor OtherActor)
    (else
      (Variables|Default|SetCombo 0))))