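; Shopmode runs the game's shop, showing a Shop widget and the mouse cursor on BeginPlay.
; It binds BuyingItem to the widget's BuyingItem1 dispatcher on every Tick rather than once at startup.
; When Level is 1, BuyingItem maps the widget's ItemNumber1 to Bear, Globe or Statue, then stores and prints that name, with no other levels handled.
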(event Custom|Buying%20Item
  (bind _asshop (Utilities|Casting|CastToShop (stale EventBeginPlay _returnvalue_2)))
  ;[1 1 1] Where it chooses what button does what
  (if (and (== (Variables|Default|GetLevel) 1) (== 1 (Variables|/Game/Blueprints/ShopBlueprints/Shop.Shop_C|GetItem%20Number%201 _asshop)))
    (bind _output_get (Variables|Default|SetBoughtItem1 "Bear"))
    (Development|PrintString _output_get)
    (elif (and (== (Variables|Default|GetLevel) 1) (== 2 (Variables|/Game/Blueprints/ShopBlueprints/Shop.Shop_C|GetItem%20Number%201 _asshop)))
      (bind _output_get_2 (Variables|Default|SetBoughtItem1 "Globe"))
      (Development|PrintString _output_get_2)
      (elif (and (== (Variables|Default|GetLevel) 1) (== 3 (Variables|/Game/Blueprints/ShopBlueprints/Shop.Shop_C|GetItem%20Number%201 _asshop)))
        (bind _output_get_3 (Variables|Default|SetBoughtItem1 "Statue"))
        (Development|PrintString _output_get_3)))))

(event EventBeginPlay
  (bind _returnvalue (Game|GetPlayerController 0))
  (bind _returnvalue_2 (UserInterface|CreateWidget "/Game/Blueprints/ShopBlueprints/Shop.Shop_C" _returnvalue))
  (UserInterface|Viewport|AddtoViewport _returnvalue_2 0)
  (Variables|/Script/Engine.PlayerController|SetbShowMouseCursor _returnvalue true))

(event EventTick
  (params (DeltaSeconds :type Float%20%28single-precision%29))
  (EventDispatchers|BindEventtoBuyingItem1Dispatcher (stale EventBeginPlay _returnvalue_2) (delegate Custom|Buying%20Item)))

(fn ConstructionScript)