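; Shop souvenir display Blueprint that reveals one souvenir component based on level and item boolean flags.
; Every Tick it picks the first true flag among three levels, then the first true flag among that level's three items.
; The matching component, such as a penguin, trophy or bear, is made visible.
; Nothing here sets the flags or hides a souvenir once shown.
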(event Collision|EventActorBeginOverlap
  (params (OtherActor :type Actor%20Object%20Reference)))

(event EventBeginPlay)

(event EventTick
  (params (DeltaSeconds :type Float%20%28single-precision%29))
  (if (Variables|Default|GetLevel%201)
    (if (Variables|Default|GetItem%2011)
      (bind _output_get (Variables|Default|Setpin (Variables|Default|Getpin)))
      (Rendering|SetVisibility _output_get true false)
      (elif (Variables|Default|GetItem%2012)
        (bind _output_get_2 (Variables|Default|Setpenguin (Variables|Default|Getpenguin)))
        (Rendering|SetVisibility _output_get_2 true false)
        (elif (Variables|Default|GetItem%2013)
          (bind _output_get_3 (Variables|Default|Setglobe (Variables|Default|Getglobe)))
          (Rendering|SetVisibility _output_get_3 true false))))
    (elif (Variables|Default|GetLevel%202)
      (if (Variables|Default|GetItem%2021)
        (bind _output_get_4 (Variables|Default|Setbowling_pin (Variables|Default|Getbowling_pin)))
        (Rendering|SetVisibility _output_get_4 true false)
        (elif (Variables|Default|GetItem%2022)
          (bind _output_get_5 (Variables|Default|Setplank (Variables|Default|Getplank)))
          (Rendering|SetVisibility _output_get_5 true false)
          (elif (Variables|Default|GetItem%2023)
            (bind _output_get_6 (Variables|Default|Settrophy (Variables|Default|Gettrophy)))
            (Rendering|SetVisibility _output_get_6 true false))))
      (elif (Variables|Default|GetLevel%203)
        (if (Variables|Default|GetItem%2031)
          (bind _output_get_7 (Variables|Default|Setfidget_cube (Variables|Default|Getfidget_cube)))
          (Rendering|SetVisibility _output_get_7 true false)
          (elif (Variables|Default|GetItem%2032)
            (bind _output_get_8 (Variables|Default|Setbear (Variables|Default|Getbear)))
            (Rendering|SetVisibility _output_get_8 true false)
            (elif (Variables|Default|GetItem%2033)
              (bind _output_get_9 (Variables|Default|Setmask (Variables|Default|Getmask)))
              (Rendering|SetVisibility _output_get_9 true false))))))))

(fn ConstructionScript)