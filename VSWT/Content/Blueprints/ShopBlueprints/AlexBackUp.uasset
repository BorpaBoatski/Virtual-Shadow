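; Backup graph of souvenir shop logic, with sections labelled SouvenirBP, LevelBP and ShopSouvenir.
; BeginPlay sets level and item flags by Level, then shows the Shop widget and mouse cursor.
; Tick rebinds the widget's purchase dispatcher to BuyingItem, which maps level and item number to a printed name and flag.
; Custom events reveal souvenir meshes from those flags, with unfinished branches and disconnected older logic left in.
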(event Custom|Buying%20Item
  ;[1 1 1] LevelBP
  (bind _asshop (Utilities|Casting|CastToShop (stale EventBeginPlay _returnvalue_2)))
  (if (== (Variables|Default|GetLevel) 1)
    (if (== 1 (Variables|/Game/Blueprints/ShopBlueprints/Shop.Shop_C|GetItem%20Number%201 _asshop))
      (bind _output_get (Variables|Default|SetBoughtItem1 "Cap"))
      (Development|PrintString _output_get)
      (Variables|/Game/Blueprints/ShopBlueprints/Souvenir.Souvenir_C|SetItem%201 "Literal" true)
      (elif (== 2 (Variables|/Game/Blueprints/ShopBlueprints/Shop.Shop_C|GetItem%20Number%201 _asshop))
        (bind _output_get_2 (Variables|Default|SetBoughtItem1 "Globe"))
        (Development|PrintString _output_get_2)
        (Variables|/Game/Blueprints/ShopBlueprints/Souvenir.Souvenir_C|SetItem%202 "Literal" true)
        (elif (== 3 (Variables|/Game/Blueprints/ShopBlueprints/Shop.Shop_C|GetItem%20Number%201 _asshop))
          (bind _output_get_3 (Variables|Default|SetBoughtItem1 "Pin"))
          (Development|PrintString _output_get_3)
          (Variables|/Game/Blueprints/ShopBlueprints/Souvenir.Souvenir_C|SetItem%203 "Literal" true))))
    (elif (== (Variables|Default|GetLevel) 2)
      (if (== 1 (Variables|/Game/Blueprints/ShopBlueprints/Shop.Shop_C|GetItem%20Number%201 _asshop))
        (bind _output_get_4 (Variables|Default|SetBoughtItem1 "Bear"))
        (Development|PrintString _output_get_4)
        (Variables|/Game/Blueprints/ShopBlueprints/Souvenir.Souvenir_C|SetItem%201 "Literal" true)
        (elif (== 2 (Variables|/Game/Blueprints/ShopBlueprints/Shop.Shop_C|GetItem%20Number%201 _asshop))
          (bind _output_get_5 (Variables|Default|SetBoughtItem1 "Penguin"))
          (Development|PrintString _output_get_5)
          (Variables|/Game/Blueprints/ShopBlueprints/Souvenir.Souvenir_C|SetItem%202 "Literal" true)
          (elif (== 3 (Variables|/Game/Blueprints/ShopBlueprints/Shop.Shop_C|GetItem%20Number%201 _asshop))
            (bind _output_get_6 (Variables|Default|SetBoughtItem1 "Sticker"))
            (Development|PrintString _output_get_6)
            (Variables|/Game/Blueprints/ShopBlueprints/Souvenir.Souvenir_C|SetItem%203 "Literal" true))))
      (elif (== (Variables|Default|GetLevel) 3)
        (if (== 1 (Variables|/Game/Blueprints/ShopBlueprints/Shop.Shop_C|GetItem%20Number%201 _asshop))
          (bind _output_get_7 (Variables|Default|SetBoughtItem1 "Somethign 1"))
          (Development|PrintString _output_get_7)
          (Variables|/Game/Blueprints/ShopBlueprints/Souvenir.Souvenir_C|SetItem%201 "Literal" true)
          (elif (== 2 (Variables|/Game/Blueprints/ShopBlueprints/Shop.Shop_C|GetItem%20Number%201 _asshop))
            (bind _output_get_8 (Variables|Default|SetBoughtItem1 "Somethign 2"))
            (Development|PrintString _output_get_8)
            (Variables|/Game/Blueprints/ShopBlueprints/Souvenir.Souvenir_C|SetItem%202 "Literal" true)
            (elif (== 3 (Variables|/Game/Blueprints/ShopBlueprints/Shop.Shop_C|GetItem%20Number%201 _asshop))
              (bind _output_get_9 (Variables|Default|SetBoughtItem1 "Something 3"))
              (Development|PrintString _output_get_9)
              (Variables|/Game/Blueprints/ShopBlueprints/Souvenir.Souvenir_C|SetItem%203 "Literal" true))))))))

(event Custom|CustomEvent
  (params (DeltaSeconds :type Float%20%28single-precision%29))
  ;[1 1 1] SouvenirBP
  (bind _asshop_souvenirs (Utilities|Casting|CastToShopSouvenirs (stale Custom|CustomEvent_1 _array_element)))
  (if (Variables|/Game/Blueprints/ShopBlueprints/ShopSouvenirs.ShopSouvenirs_C|GetLevel%201 _asshop_souvenirs)
    (if (Variables|Default|GetItem%201)
      (Variables|Default|Setcap (Variables|Default|Getcap))
      (Rendering|SetVisibility (Variables|Default|Getcap) true false)
      (elif (Variables|Default|GetItem%202)
        (Variables|Default|Setglobe (Variables|Default|Getglobe))
        (Rendering|SetVisibility (Variables|Default|Getglobe) true false)
        (elif (Variables|Default|GetItem%203)
          (Variables|Default|Setbowling_pin (Variables|Default|Getbowling_pin))
          (Rendering|SetVisibility (Variables|Default|Getbowling_pin) true false))))
    (elif (Variables|/Game/Blueprints/ShopBlueprints/ShopSouvenirs.ShopSouvenirs_C|GetLevel%202 _asshop_souvenirs)
      (if (not (Variables|Default|GetItem%201))
        (if (not (Variables|Default|GetItem%202))
          (if (Variables|Default|GetItem%203)
            _)))
      (elif (Variables|/Game/Blueprints/ShopBlueprints/ShopSouvenirs.ShopSouvenirs_C|GetLevel%203 _asshop_souvenirs)
        (if (not (Variables|Default|GetItem%201))
          (if (not (Variables|Default|GetItem%202))
            (if (Variables|Default|GetItem%203)
              _)))))))

(event Custom|CustomEvent_1
  ;[1 1 1] SouvenirBP
  (bind _outactors (Actor|GetAllActorsOfClass "/Game/Blueprints/ShopBlueprints/ShopSouvenirs.ShopSouvenirs_C"))
  (for _array_element _outactors
    (bind _asshop_souvenirs (Utilities|Casting|CastToShopSouvenirs _array_element))
    (if (Variables|/Game/Blueprints/ShopBlueprints/ShopSouvenirs.ShopSouvenirs_C|GetLevel%201 _asshop_souvenirs)
      (if (Variables|Default|GetItem%201)
        (Variables|Default|Setcap (Variables|Default|Getcap))
        (Rendering|SetVisibility (Variables|Default|Getcap) true false)
        (elif (Variables|Default|GetItem%202)
          (Variables|Default|Setglobe (Variables|Default|Getglobe))
          (Rendering|SetVisibility (Variables|Default|Getglobe) true false)
          (elif (Variables|Default|GetItem%203)
            (Variables|Default|Setbowling_pin (Variables|Default|Getbowling_pin))
            (Rendering|SetVisibility (Variables|Default|Getbowling_pin) true false))))
      (elif (Variables|/Game/Blueprints/ShopBlueprints/ShopSouvenirs.ShopSouvenirs_C|GetLevel%202 _asshop_souvenirs)
        (if (not (Variables|Default|GetItem%201))
          (if (not (Variables|Default|GetItem%202))
            (if (Variables|Default|GetItem%203)
              _)))
        (elif (Variables|/Game/Blueprints/ShopBlueprints/ShopSouvenirs.ShopSouvenirs_C|GetLevel%203 _asshop_souvenirs)
          (if (not (Variables|Default|GetItem%201))
            (if (not (Variables|Default|GetItem%202))
              (if (Variables|Default|GetItem%203)
                _))))))))

(event Custom|CustomEvent_2
  ;[1 1 1] ShopSouvenir
)

(event Custom|CustomEvent_3
  (params (DeltaSeconds :type Float%20%28single-precision%29))
  ;[1 1 1] ShopSouvenir
  (if (Variables|Default|GetLevel%201)
    (if (Variables|Default|GetItem%2011)
      (bind _output_get (Variables|Default|Setcap (Variables|Default|Getcap)))
      (Rendering|SetVisibility _output_get true false)
      (elif (Variables|Default|GetItem%2012)
        (bind _output_get_2 (Variables|Default|Setglobe (Variables|Default|Getglobe)))
        (Rendering|SetVisibility _output_get_2 true false)
        (elif (Variables|Default|GetItem%2013)
          (bind _output_get_3 (Variables|Default|Setbowling_pin (Variables|Default|Getbowling_pin)))
          (Rendering|SetVisibility _output_get_3 true false))))
    (elif (Variables|Default|GetLevel%202)
      (if (Variables|Default|GetItem%2021)
        (bind _output_get_4 (Variables|Default|SetCone (Variables|Default|GetCone)))
        (Rendering|SetVisibility _output_get_4 true false)
        (elif (Variables|Default|GetItem%2022)
          (bind _output_get_5 (Variables|Default|SetSphere (Variables|Default|GetSphere)))
          (Rendering|SetVisibility _output_get_5 true false)
          (elif (Variables|Default|GetItem%2023)
            (bind _output_get_6 (Variables|Default|SetCube (Variables|Default|GetCube)))
            (Rendering|SetVisibility _output_get_6 true false))))
      (elif (Variables|Default|GetLevel%203)
        (if (Variables|Default|GetItem%2031)
          (bind _output_get_7 (Variables|Default|SetCylinder (Variables|Default|GetCylinder)))
          (Rendering|SetVisibility _output_get_7 true false)
          (elif (Variables|Default|GetItem%2032)
            (bind _output_get_8 (Variables|Default|Setglobe (Variables|Default|Getglobe)))
            (Rendering|SetVisibility _output_get_8 true false)
            (elif (Variables|Default|GetItem%2033)
              (bind _output_get_9 (Variables|Default|Setbowling_pin (Variables|Default|Getbowling_pin)))
              (Rendering|SetVisibility _output_get_9 true false))))))))

(event Collision|EventActorBeginOverlap
  (params (OtherActor :type Actor%20Object%20Reference))
  ;[1 1 1] ShopSouvenir
)

(event EventTick
  (params (DeltaSeconds :type Float%20%28single-precision%29))
  ;[1 1 1] LevelBP
  (EventDispatchers|BindEventtoBuyingItem1Dispatcher (stale EventBeginPlay _returnvalue_2) (delegate Custom|Buying%20Item)))

(event EventBeginPlay
  (bind _returnvalue (Game|GetPlayerController 0))
  ;[1 1 1] LevelBP
  ;;[1 1 1] Originally This connects to Create Shop Widget
  ;;[1 1 1] Chooses whats in the shop
  (if (== (Variables|Default|GetLevel) 1)
    (Variables|/Game/Blueprints/ShopBlueprints/ShopSouvenirs.ShopSouvenirs_C|SetItem%2011 "Literal" true)
    (Variables|/Game/Blueprints/ShopBlueprints/ShopSouvenirs.ShopSouvenirs_C|SetItem%2012 "Literal" true)
    (Variables|/Game/Blueprints/ShopBlueprints/ShopSouvenirs.ShopSouvenirs_C|SetItem%2013 "Literal" true)
    (Variables|/Game/Blueprints/ShopBlueprints/ShopSouvenirs.ShopSouvenirs_C|SetLevel%201 "Literal" true)
    (Variables|/Game/Blueprints/ShopBlueprints/ShopSouvenirs.ShopSouvenirs_C|SetLevel%201 "Literal" true)
    (Variables|/Game/Blueprints/ShopBlueprints/ShopSouvenirs.ShopSouvenirs_C|SetLevel%201 "Literal" true)
    (bind _returnvalue_2 (UserInterface|CreateWidget "/Game/Blueprints/ShopBlueprints/Shop.Shop_C" _returnvalue :!label _label))
    (UserInterface|Viewport|AddtoViewport _returnvalue_2 0)
    (Variables|/Script/Engine.PlayerController|SetbShowMouseCursor _returnvalue true)
    (elif (== (Variables|Default|GetLevel) 2)
      (Variables|/Game/Blueprints/ShopBlueprints/ShopSouvenirs.ShopSouvenirs_C|SetItem%2021 "Literal" true)
      (Variables|/Game/Blueprints/ShopBlueprints/ShopSouvenirs.ShopSouvenirs_C|SetItem%2022 "Literal" true)
      (Variables|/Game/Blueprints/ShopBlueprints/ShopSouvenirs.ShopSouvenirs_C|SetItem%2023 "Literal" true)
      (Variables|/Game/Blueprints/ShopBlueprints/ShopSouvenirs.ShopSouvenirs_C|SetLevel%202 "Literal" true)
      (Variables|/Game/Blueprints/ShopBlueprints/ShopSouvenirs.ShopSouvenirs_C|SetLevel%202 "Literal" true)
      (Variables|/Game/Blueprints/ShopBlueprints/ShopSouvenirs.ShopSouvenirs_C|SetLevel%202 "Literal" true)
      (goto _label)
      (elif (== (Variables|Default|GetLevel) 3)
        (Variables|/Game/Blueprints/ShopBlueprints/ShopSouvenirs.ShopSouvenirs_C|SetItem%2031 "Literal" true)
        (Variables|/Game/Blueprints/ShopBlueprints/ShopSouvenirs.ShopSouvenirs_C|SetItem%2032 "Literal" true)
        (Variables|/Game/Blueprints/ShopBlueprints/ShopSouvenirs.ShopSouvenirs_C|SetItem%2033 "Literal" true)
        (Variables|/Game/Blueprints/ShopBlueprints/ShopSouvenirs.ShopSouvenirs_C|SetLevel%203 "Literal" true)
        (Variables|/Game/Blueprints/ShopBlueprints/ShopSouvenirs.ShopSouvenirs_C|SetLevel%203 "Literal" true)
        (Variables|/Game/Blueprints/ShopBlueprints/ShopSouvenirs.ShopSouvenirs_C|SetLevel%203 "Literal" true)
        (goto _label)))))

(event Input|KeyboardEvents|SpaceBar
  (params (Key :type Key%20Structure))
  ;[1 1 1] LevelBP
  (:Pressed
    (bind _output_get (Variables|Default|SetShopStart true))
    (if _output_get
      _)))

(fn ConstructionScript)