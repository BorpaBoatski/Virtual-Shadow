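; Rhythm game board that spawns notes across four lanes and tracks points, combo and health, adding a HUD on start.
; Tick compares game time to a hard-coded time-to-lane map, spawning and removing each note with a fixed lead time.
; D/F/J/K lift plucks, enabling overlaps only during the move; hits score by proximity, with combo multiplying the whole running total.
; Notes reaching DeadEnd cost health and reset combo.
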(event OnComponentBeginOverlap(DeadEnd)
  (params (OverlappedComponent :type Primitive%20Component%20Object%20Reference) (OtherActor :type Actor%20Object%20Reference) (OtherComp :type Primitive%20Component%20Object%20Reference) (OtherBodyIndex :type Integer) (bFromSweep :type Boolean) (SweepResult :type Hit%20Result%20Structure%20%28by%20ref%29))
  ;[1 1 1] Health System
  (if (== (Utilities|GetClass OtherActor) "/Game/Blueprints/Note_BP.Note_BP_C")
    (Variables|Default|SetHealth (- (Variables|Default|GetHealth) 1.0))
    (Variables|Default|SetCombo 0)
    (Actor|DestroyActor OtherActor)))

(event OnComponentBeginOverlap(Pluck1)
  (params (OverlappedComponent :type Primitive%20Component%20Object%20Reference) (OtherActor :type Actor%20Object%20Reference) (OtherComp :type Primitive%20Component%20Object%20Reference) (OtherBodyIndex :type Integer) (bFromSweep :type Boolean) (SweepResult :type Hit%20Result%20Structure%20%28by%20ref%29))
  ;[1 1 1] Pluck 1 Detection
  (if (== (Utilities|GetClass OtherActor) "/Game/Blueprints/Note_BP.Note_BP_C")
    (bind _output_get (Variables|Default|SetCombo (+ (Variables|Default|GetCombo) 1)))
    (Variables|Default|SetPoints (* (+ (Variables|Default|GetPoints) (Math|Float|Truncate (/ (Variables|Default|GetMaxPoint) (Math|Vector|VectorLength (- (Transformation|GetActorLocation OtherActor) (Transformation|GetWorldLocation (Variables|Default|GetPluck1))))))) _output_get))
    (Actor|DestroyActor OtherActor)))

(event OnComponentBeginOverlap(Pluck2)
  (params (OverlappedComponent :type Primitive%20Component%20Object%20Reference) (OtherActor :type Actor%20Object%20Reference) (OtherComp :type Primitive%20Component%20Object%20Reference) (OtherBodyIndex :type Integer) (bFromSweep :type Boolean) (SweepResult :type Hit%20Result%20Structure%20%28by%20ref%29))
  ;[1 1 1] Pluck 2 Detection
  (if (== (Utilities|GetClass OtherActor) "/Game/Blueprints/Note_BP.Note_BP_C")
    (bind _output_get (Variables|Default|SetCombo (+ (Variables|Default|GetCombo) 1)))
    (Variables|Default|SetPoints (* (+ (Variables|Default|GetPoints) (Math|Float|Truncate (/ (Variables|Default|GetMaxPoint) (Math|Vector|VectorLength (- (Transformation|GetActorLocation OtherActor) (Transformation|GetWorldLocation (Variables|Default|GetPluck2))))))) _output_get))
    (Actor|DestroyActor OtherActor)))

(event OnComponentBeginOverlap(Pluck3)
  (params (OverlappedComponent :type Primitive%20Component%20Object%20Reference) (OtherActor :type Actor%20Object%20Reference) (OtherComp :type Primitive%20Component%20Object%20Reference) (OtherBodyIndex :type Integer) (bFromSweep :type Boolean) (SweepResult :type Hit%20Result%20Structure%20%28by%20ref%29))
  ;[1 1 1] Pluck 3 Detection
  (if (== (Utilities|GetClass OtherActor) "/Game/Blueprints/Note_BP.Note_BP_C")
    (bind _output_get (Variables|Default|SetCombo (+ (Variables|Default|GetCombo) 1)))
    (Variables|Default|SetPoints (* (+ (Variables|Default|GetPoints) (Math|Float|Truncate (/ (Variables|Default|GetMaxPoint) (Math|Vector|VectorLength (- (Transformation|GetActorLocation OtherActor) (Transformation|GetWorldLocation (Variables|Default|GetPluck3))))))) _output_get))
    (Actor|DestroyActor OtherActor)))

(event OnComponentBeginOverlap(Pluck4)
  (params (OverlappedComponent :type Primitive%20Component%20Object%20Reference) (OtherActor :type Actor%20Object%20Reference) (OtherComp :type Primitive%20Component%20Object%20Reference) (OtherBodyIndex :type Integer) (bFromSweep :type Boolean) (SweepResult :type Hit%20Result%20Structure%20%28by%20ref%29))
  ;[1 1 1] Pluck 4 Detection
  (if (== (Utilities|GetClass OtherActor) "/Game/Blueprints/Note_BP.Note_BP_C")
    (bind _output_get (Variables|Default|SetCombo (+ (Variables|Default|GetCombo) 1)))
    (Variables|Default|SetPoints (* (+ (Variables|Default|GetPoints) (Math|Float|Truncate (/ (Variables|Default|GetMaxPoint) (Math|Vector|VectorLength (- (Transformation|GetActorLocation OtherActor) (Transformation|GetWorldLocation (Variables|Default|GetPluck4))))))) _output_get))
    (Actor|DestroyActor OtherActor)))

(event EventBeginPlay
  ;[1 1 1] Init
  (CallFunction|GetSpawnPoints)
  (CallFunction|GetScore)
  (bind _returnvalue (UserInterface|CreateWidget "/Game/Blueprints/Rhythm_HUD.Rhythm_HUD_C" (Game|GetPlayerController 0)))
  (UserInterface|Viewport|AddtoViewport _returnvalue 0))

(event EventTick
  (params (DeltaSeconds :type Float%20%28single-precision%29))
  (bind _musicscore (Variables|Default|GetMusicScore))
  ;[1 1 1] Spawn when timing is reached
  (bind _output_get (Variables|Default|SetSongPosition (Utilities|Time|GetTimeSeconds)))
  (if (> (Utilities|Map|Length (Variables|Default|GetMusicScore)) 0)
    (bind _keys (Utilities|Map|Keys _musicscore))
    (if (>= _output_get (- (Utilities|Array|Get(acopy) _keys) 2.8))
      (CallFunction|SpawnNote (.Value (Utilities|Map|Find _musicscore (Utilities|Array|Get(acopy) _keys)))))))

(event Input|KeyboardEvents|K
  (params (Key :type Key%20Structure))
  (bind _pluck4 (Variables|Default|GetPluck4))
  (bind _pluck4_2 (Variables|Default|GetPluck4))
  ;[1 1 1] Lift/Drop Pluck4
  (:Pressed
    (Variables|/Script/Engine.PrimitiveComponent|SetbGenerateOverlapEvents _pluck4 true)
    (Transformation|SetWorldLocation _pluck4 (+ (Transformation|GetWorldLocation _pluck4) "0,0.000000,30.000000") false false)
    (Variables|/Script/Engine.PrimitiveComponent|SetbGenerateOverlapEvents _pluck4 false))
  (:Released
    (Variables|/Script/Engine.PrimitiveComponent|SetbGenerateOverlapEvents _pluck4_2 false)
    (Transformation|SetWorldLocation _pluck4_2 (+ (Transformation|GetWorldLocation _pluck4_2) "0,0.000000,-30.000000") false false)))

(event Input|KeyboardEvents|D
  (params (Key :type Key%20Structure))
  (bind _pluck1 (Variables|Default|GetPluck1))
  (bind _pluck1_2 (Variables|Default|GetPluck1))
  ;[1 1 1] Lift/Drop Pluck1
  (:Pressed
    (Variables|/Script/Engine.PrimitiveComponent|SetbGenerateOverlapEvents _pluck1 true)
    (Transformation|SetWorldLocation _pluck1 (+ (Transformation|GetWorldLocation _pluck1) "0,0.000000,30.000000") false false)
    (Variables|/Script/Engine.PrimitiveComponent|SetbGenerateOverlapEvents _pluck1 false))
  (:Released
    (Variables|/Script/Engine.PrimitiveComponent|SetbGenerateOverlapEvents _pluck1_2 false)
    (Transformation|SetWorldLocation _pluck1_2 (+ (Transformation|GetWorldLocation _pluck1_2) "0,0.000000,-30.000000") false false)))

(event Input|KeyboardEvents|J
  (params (Key :type Key%20Structure))
  (bind _pluck3 (Variables|Default|GetPluck3))
  (bind _pluck3_2 (Variables|Default|GetPluck3))
  ;[1 1 1] Lift/Drop Pluck3
  (:Pressed
    (Variables|/Script/Engine.PrimitiveComponent|SetbGenerateOverlapEvents _pluck3 true)
    (Transformation|SetWorldLocation _pluck3 (+ (Transformation|GetWorldLocation _pluck3) "0,0.000000,30.000000") false false)
    (Variables|/Script/Engine.PrimitiveComponent|SetbGenerateOverlapEvents _pluck3 false))
  (:Released
    (Variables|/Script/Engine.PrimitiveComponent|SetbGenerateOverlapEvents _pluck3_2 false)
    (Transformation|SetWorldLocation _pluck3_2 (+ (Transformation|GetWorldLocation _pluck3_2) "0,0.000000,-30.000000") false false)))

(event Input|KeyboardEvents|F
  (params (Key :type Key%20Structure))
  (bind _pluck2 (Variables|Default|GetPluck2))
  (bind _pluck2_2 (Variables|Default|GetPluck2))
  ;[1 1 1] Lift/Drop Pluck2
  (:Pressed
    (Variables|/Script/Engine.PrimitiveComponent|SetbGenerateOverlapEvents _pluck2 true)
    (Transformation|SetWorldLocation _pluck2 (+ (Transformation|GetWorldLocation _pluck2) "0,0.000000,30.000000") false false)
    (Variables|/Script/Engine.PrimitiveComponent|SetbGenerateOverlapEvents _pluck2 false))
  (:Released
    (Variables|/Script/Engine.PrimitiveComponent|SetbGenerateOverlapEvents _pluck2_2 false)
    (Transformation|SetWorldLocation _pluck2_2 (+ (Transformation|GetWorldLocation _pluck2_2) "0,0.000000,-30.000000") false false)))

(fn ConstructionScript)

(fn GetSpawnPoints
  (Variables|Default|SetSpawnPoints (Utilities|Array|MakeArray (Transformation|GetWorldTransform (Variables|Default|GetArrow1)) (Transformation|GetWorldTransform (Variables|Default|GetArrow2)) (Transformation|GetWorldTransform (Variables|Default|GetArrow3)) (Transformation|GetWorldTransform (Variables|Default|GetArrow4)))))

(fn SpawnNote
  (params (SpawnPoint :type Integer))
  (bind _musicscore (Variables|Default|GetMusicScore))
  (Game|SpawnActorfromClass "/Game/Blueprints/Note_BP.Note_BP_C" (Utilities|Array|Get(acopy) (Variables|Default|GetSpawnPoints) SpawnPoint) "Undefined" 0 0)
  (if (> (Utilities|Map|Length (Variables|Default|GetMusicScore)) 0)
    (bind _keys (Utilities|Map|Keys _musicscore))
    (Utilities|Map|Remove _musicscore (Utilities|Array|Get(acopy) _keys))))

(fn GetScore
  (Variables|Default|SetMusicScore (Utilities|Map|MakeMap 12.0 0 13.7 1 14.6 2 15.0 3)))