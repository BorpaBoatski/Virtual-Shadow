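; Signpost actor that shows its own text in an on-screen dialogue widget when interacted with.
; The Interact event works as a toggle: it creates the widget for the first player and fills it with MyText, or removes it if already open.
; When the third-person character leaves the Box component, the widget is removed and its reference cleared, without a validity check.
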(event OnComponentEndOverlap(Box)
  (params (OverlappedComponent :type Primitive%20Component%20Object%20Reference) (OtherActor :type Actor%20Object%20Reference) (OtherComp :type Primitive%20Component%20Object%20Reference) (OtherBodyIndex :type Integer))
  (Utilities|Casting|CastToThirdPersonCharacter OtherActor)
  (Widget|RemovefromParent (Variables|Default|GetDialogueWidget))
  (Variables|Default|SetDialogueWidget 0))

(event EventBeginPlay)

(event Collision|EventActorBeginOverlap
  (params (OtherActor :type Actor%20Object%20Reference)))

(event EventTick
  (params (DeltaSeconds :type Float%20%28single-precision%29)))

(event EventInteract
  (Utilities|IsValid (Variables|Default|GetDialogueWidget)
    (:Is%20Valid
      (Widget|RemovefromParent (Variables|Default|GetDialogueWidget))
      (Variables|Default|SetDialogueWidget 0))
    (:Is%20Not%20Valid
      (bind _returnvalue (UserInterface|CreateWidget "/Game/Dialogue/DialogueWidget.DialogueWidget_C" (Game|GetPlayerController 0)))
      (bind _output_get (Variables|Default|SetDialogueWidget _returnvalue))
      (UserInterface|Viewport|AddtoViewport _output_get 0)
      (Variables|/Game/Dialogue/DialogueWidget.DialogueWidget_C|SetDialogueText (Variables|Default|GetDialogueWidget) (Variables|Default|GetMyText)))))

(fn ConstructionScript)