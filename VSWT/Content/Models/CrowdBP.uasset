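; CrowdBP is a crowd member Blueprint whose physics-driven CrowdModel hops repeatedly.
; BeginPlay starts a looping one-second timer that calls Jump, which adds a small upward linear velocity and prints a debug string.
; ChangeColor builds a red dynamic material instance but calls SetMaterial without passing it.
; Nothing in the file calls ChangeColor, and the ChangeMatColor event is empty.
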(event Custom|ChangeMatColor)

(event EventBeginPlay
  (Utilities|Time|SetTimerbyFunctionName 0 "Jump" 1.0 true))

(fn ConstructionScript)

(fn ChangeColor
  (bind _returnvalue (Rendering|Material|CreateDynamicMaterialInstance (Rendering|Material|GetMaterial (Variables|Default|GetCrowdModel) 0) "None" :!class /Script/Engine.KismetMaterialLibrary))
  (Rendering|Material|SetVectorParameterValue _returnvalue "Crowd_Mat" "(R=0.654167,G=0.032066,B=0.000000,A=1.000000)" :!class /Script/Engine.MaterialInstanceDynamic)
  (Rendering|Material|SetMaterial (Variables|Default|GetCrowdModel) 0 0)
  (Development|PrintString "Changed!"))

(fn Jump
  (Physics|SetPhysicsLinearVelocity (Variables|Default|GetCrowdModel) "0, 0,10.000000" true "None")
  (Development|PrintString "Jumo"))