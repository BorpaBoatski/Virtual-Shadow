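; BP_RoadSpawner creates an endless road along the Y axis by recycling existing ground actors rather than spawning new ones.
; Each Tick, it compares the Bus's Y position with the current entry in the GrountSets array.
; Once the bus is at least TileYSize ahead, that piece jumps forward two tile lengths.
; The current index then advances, wrapping to zero at the array's end.
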(event EventBeginPlay)

(event EventTick
  (params (DeltaSeconds :type Float%20%28single-precision%29))
  (bind _grountsets (Variables|Default|GetGrountSets))
  (if (>= (- (.Y (Math|Vector|BreakVector (Transformation|GetActorLocation (Variables|Default|GetBus)))) (.Y (Math|Vector|BreakVector (Transformation|GetActorLocation (Utilities|Array|Get(acopy) (Variables|Default|GetGrountSets) (Variables|Default|GetCurrentGroundIndex)))))) (Variables|Default|GetTileYSize))
    (Transformation|SetActorLocation (Utilities|Array|Get(acopy) _grountsets (Variables|Default|GetCurrentGroundIndex)) (+ (Transformation|GetActorLocation (Utilities|Array|Get(acopy) _grountsets (Variables|Default|GetCurrentGroundIndex))) (Math|Vector|MakeVector 0.0 (* (Variables|Default|GetTileYSize) 2.0) 0.0)) false false)
    ;[1 1 1] Prevent array out of bound
    (bind _result (Math|Integer|IncrementInt (Variables|Default|GetCurrentGroundIndex))
      (:%20%20
        (if (>= _result (Utilities|Array|Length _grountsets))
          (Variables|Default|SetCurrentGroundIndex 0))))))

(fn ConstructionScript)